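; Obstacle block for a runner game that costs the player a life on contact.
; When a ThirdPersonCharacter overlaps it, it decrements Life on the ThirdPersonGameMode, waits briefly, then spawns an explosion and crash sound and destroys itself.
; It then calls the character's DeathFunction if Life has dropped below zero.
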(event EventBeginPlay)

(event Collision|EventActorBeginOverlap
  (params (OtherActor :type Actor%20Object%20Reference))
  (Utilities|Casting|CastToThirdPersonCharacter OtherActor)
  (bind _asthird_person_game_mode (Utilities|Casting|CastToThirdPersonGameMode (Game|GetGameMode)))
  (Math|Integer|DecrementInt (Variables|/Game/ThirdPersonBP/Blueprints/ThirdPersonGameMode.ThirdPersonGameMode_C|GetLife _asthird_person_game_mode)
    (:%20%20
      (Utilities|FlowControl|Delay 0.2)
      (Effects|SpawnEmitteratLocation "/Game/MobileStarterContent/Particles/P_Explosion.P_Explosion" (Transformation|GetActorLocation) "0, 0, 0" "5.000000,5.000000,5.000000")
      (Audio|SpawnSound2D "/Game/RunnerFiles/SFX/barricadeCrash.barricadeCrash" 1.0 1.0 0.0 0)
      (Actor|DestroyActor)
      (bind _asthird_person_game_mode_2 (Utilities|Casting|CastToThirdPersonGameMode (Game|GetGameMode)))
      (if (< (Variables|/Game/ThirdPersonBP/Blueprints/ThirdPersonGameMode.ThirdPersonGameMode_C|GetLife _asthird_person_game_mode_2) 0)
        (bind _asthird_person_character (Utilities|Casting|CastToThirdPersonCharacter OtherActor))
        (Default|DeathFunction _asthird_person_character)))))

(event EventTick
  (params (DeltaSeconds :type Float%20%28single-precision%29)))

(fn ConstructionScript)